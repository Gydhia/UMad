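; ArrowBP is an arrow projectile that acts as a trap hazard for the KahnaxChar character.
; Tick accumulates elapsed time and destroys the actor once it reaches LifeTime.
; On Hit, it compares the other actor to the first KahnaxChar found in the world and, on a match, calls HitByTrap with the arrow component's velocity scaled up tenfold.
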(event `self.ReceiveBeginPlay`
  (set `self.life` 0.0))

(event `self.ReceiveTick`
  (params (DeltaSeconds :type "Float (single-precision)"))
  (bind _life (`self.life`))
  (set `self.life` (+ _life DeltaSeconds))
  (if (>= _life (`self.lifeTime`))
    (`self.K2_DestroyActor`)))

(event `self.ReceiveHit`
  (params (MyComp :type "PrimitiveComponent Object Reference") (Other :type "Actor Object Reference") (OtherComp :type "PrimitiveComponent Object Reference") (bSelfMoved :type Boolean) (HitLocation :type "Vector Structure") (HitNormal :type "Vector Structure") (NormalImpulse :type "Vector Structure") (Hit :type "HitResult Structure (by ref)"))
  (bind _returnvalue (`GameplayStatics.GetActorOfClass` "/Game/Character/KahnaxChar.KahnaxChar_C"))
  (if (== Other _returnvalue)
    (`UMadCharacter.HitByTrap` _returnvalue (* (`SceneComponent.GetComponentVelocity` MyComp) (10.0 10.0 10.0)))))

(fn `UserConstructionScript`)