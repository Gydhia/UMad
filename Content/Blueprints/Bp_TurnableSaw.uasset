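; Moving saw trap that spins and shuttles back and forth over a set distance, hurting the KahnaxChar player on contact.
; Tick moves it along an axis-remapped Direction and reverses TravelSpeed when the timer exceeds distance over speed.
; Hit passes a scaled impulse to the player's HitByTrap.
; Trigger quadruples travel and spin speed for three seconds, rescaling the timer to keep its place along the path.
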(event `self.ReceiveBeginPlay`
  (set `self.timeTravel` 0.0)
  (set `self.timeToTravel` (/ (`self.distanceToTravel`) (`self.travelSpeed`)))
  (bind _returnvalue (`GameplayStatics.GetActorOfClass` "/Game/Character/KahnaxChar.KahnaxChar_C"))
  (set `self.player` _returnvalue))

(event `self.ReceiveTick`
  (params (DeltaSeconds :type "Float (single-precision)"))
  (bind _travelspeed (`self.travelSpeed`))
  (bind _output_get (set `self.timeTravel` (+ (`self.timeTravel`) DeltaSeconds)))
  (if (> _output_get (`self.timeToTravel`))
    (set `self.timeTravel` 0.0)
    (set `self.travelSpeed` (* (`self.travelSpeed`) -1))
    (else
      (`self.K2_SetActorTransform` (`KismetMathLibrary.MakeTransform` (+ (`KismetMathLibrary.MakeVector` (* (.y (`self.direction`)) _travelspeed DeltaSeconds -1.0) (* (.x (`self.direction`)) _travelspeed DeltaSeconds) (* (.z (`self.direction`)) _travelspeed DeltaSeconds -1.0)) (.location (`self.GetTransform`))) (.rotation (`self.GetTransform`)) (.scale (`self.GetTransform`)))))))

(event `self.ReceiveHit`
  (params (MyComp :type "PrimitiveComponent Object Reference") (Other :type "Actor Object Reference") (OtherComp :type "PrimitiveComponent Object Reference") (bSelfMoved :type Boolean) (HitLocation :type "Vector Structure") (HitNormal :type "Vector Structure") (NormalImpulse :type "Vector Structure") (Hit :type "HitResult Structure (by ref)"))
  (bind _player (`self.player`))
  (if (== Other _player)
    (`UMadCharacter.HitByTrap` _player (/ (* NormalImpulse (60.0 60.0 60.0)) (stale `self.ReceiveTick` DeltaSeconds)))))

(event `Trigger`
  (set `self.travelSpeed` (* (`self.travelSpeed`) 4.0))
  (set `self.timeTravel` (`KismetMathLibrary.Abs` (* (`self.timeTravel`) 0.25)))
  (set `self.timeToTravel` (`KismetMathLibrary.Abs` (/ (`self.distanceToTravel`) (`self.travelSpeed`))))
  (set `RotatingMovementComponent.RotationRate` (struct :`Yaw` 1440.0) (`self.RotatingMovement`))
  (`KismetSystemLibrary.Delay` 3.0)
  (set `self.travelSpeed` (* (`self.travelSpeed`) 0.25))
  (set `self.timeTravel` (`KismetMathLibrary.Abs` (* (`self.timeTravel`) 4.0)))
  (set `self.timeToTravel` (`KismetMathLibrary.Abs` (/ (`self.distanceToTravel`) (`self.travelSpeed`))))
  (set `RotatingMovementComponent.RotationRate` (struct :`Yaw` 360.0) (`self.RotatingMovement`)))

(fn `UserConstructionScript`)