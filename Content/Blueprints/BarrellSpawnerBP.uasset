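; Barrel spawner actor that stays practically idle until its Trigger event starts a five-second burst of rapid barrel spawning.
; Tick runs a cooldown derived from FireRate, which Trigger raises and then drops back to near zero after a delay.
; Each BarrelBP spawns at a random XY point in a square area centered on the spawner.
; Its Stone component receives an impulse along its negative up vector, scaled by inverse frame time.
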(event `self.ReceiveBeginPlay`
  (set `self.fireRate` 1e-06)
  (set `self.cooldown` (/ 1.0 (`self.fireRate`))))

(event `self.ReceiveTick`
  (params (DeltaSeconds :type "Float (single-precision)"))
  (bind _returnvalue (/ (`self.areaSize`) -2.0))
  (if (>= (`self.cdProgress`) (`self.cooldown`))
    (bind _returnvalue_2 (`|SpawnActorFromClass` "/Game/Blueprints/BarrelBP.BarrelBP_C" (`KismetMathLibrary.MakeTransform` (`KismetMathLibrary.MakeVector` (+ (* (`KismetMathLibrary.RandomFloat`) (`self.areaSize`)) (.x (.location (`self.GetTransform`))) _returnvalue) (+ (* (`KismetMathLibrary.RandomFloat`) (`self.areaSize`)) (.y (.location (`self.GetTransform`))) _returnvalue) (.z (.location (`self.GetTransform`)))) (.rotation (`self.GetTransform`)) (.scale (`self.GetTransform`))) "AdjustIfPossibleButAlwaysSpawn" "OverrideRootScale" self null))
    (set `self.cdProgress` 0.0)
    (bind _stone (`/Game/Blueprints/BarrelBP.Stone` _returnvalue_2))
    (`PrimitiveComponent.AddImpulse` _stone (/ (* (`KismetMathLibrary.GetUpVector` (`SceneComponent.K2_GetComponentRotation` _stone)) (`KismetMathLibrary.SelectFloat` -400.0 0.0 true)) DeltaSeconds) "None" false)
    (else
      (set `self.cdProgress` (+ DeltaSeconds (`self.cdProgress`))))))

(event `Trigger`
  (set `self.fireRate` 50.0)
  (set `self.cooldown` (/ 1.0 (`self.fireRate`)))
  (`KismetSystemLibrary.Delay` 5.0)
  (set `self.fireRate` 0.0001)
  (set `self.cooldown` (/ 1.0 (`self.fireRate`))))

(fn `UserConstructionScript`)