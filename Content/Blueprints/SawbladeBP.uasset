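; Moving sawblade trap that shuttles back and forth and knocks the player when hit.
; Tick rolls the blade and moves it perpendicular to its forward vector, reversing speed whenever the travel time derived from distance and speed elapses.
; Trigger temporarily quadruples speed, rescaling the timers to match, then restores it after a delay.
; Hit applies an impulse along the travel direction to the KahnaxChar player and calls HitByTrap.
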(event `self.ReceiveHit`
  (params (MyComp :type "PrimitiveComponent Object Reference") (Other :type "Actor Object Reference") (OtherComp :type "PrimitiveComponent Object Reference") (bSelfMoved :type Boolean) (HitLocation :type "Vector Structure") (HitNormal :type "Vector Structure") (NormalImpulse :type "Vector Structure") (Hit :type "HitResult Structure (by ref)"))
  (bind _player (`self.player`))
  (bind _travelspeed (`self.travelSpeed`))
  (if (== Other _player)
    (`PrimitiveComponent.AddImpulse` (`Character.CapsuleComponent` _player) (* (/ (`KismetMathLibrary.MakeVector` (* (.y (`KismetMathLibrary.GetForwardVector` (`SceneComponent.K2_GetComponentRotation` MyComp))) _travelspeed (stale `self.ReceiveTick` DeltaSeconds) -1.0) (* (.x (`KismetMathLibrary.GetForwardVector` (`SceneComponent.K2_GetComponentRotation` MyComp))) _travelspeed (stale `self.ReceiveTick` DeltaSeconds)) (* (.z (`KismetMathLibrary.GetForwardVector` (`SceneComponent.K2_GetComponentRotation` MyComp))) _travelspeed (stale `self.ReceiveTick` DeltaSeconds) -1.0)) (stale `self.ReceiveTick` DeltaSeconds)) (`KismetMathLibrary.SelectFloat` 4.0 0.0 true)) "None" false)
    (`/Game/Character/KahnaxChar.HitByTrap` (`self.player`))))

(event `Trigger`
  (set `self.travelSpeed` (* (`self.travelSpeed`) 4.0))
  (set `self.timeTravel` (`KismetMathLibrary.Abs` (* (`self.timeTravel`) 0.25)))
  (set `self.timeToTravel` (`KismetMathLibrary.Abs` (/ (`self.distanceToTravel`) (`self.travelSpeed`))))
  (`KismetSystemLibrary.Delay` 3.0)
  (set `self.travelSpeed` (* (`self.travelSpeed`) 0.25))
  (set `self.timeTravel` (`KismetMathLibrary.Abs` (* (`self.timeTravel`) 4.0)))
  (set `self.timeToTravel` (`KismetMathLibrary.Abs` (/ (`self.distanceToTravel`) (`self.travelSpeed`)))))

(event `self.ReceiveBeginPlay`
  (set `self.timeTravel` 0.0)
  (set `self.timeToTravel` (/ (`self.distanceToTravel`) (`self.travelSpeed`)))
  (bind _returnvalue (`GameplayStatics.GetActorOfClass` "/Game/Character/KahnaxChar.KahnaxChar_C"))
  (set `self.player` _returnvalue))

(event `self.ReceiveTick`
  (params (DeltaSeconds :type "Float (single-precision)"))
  (bind _travelspeed (`self.travelSpeed`))
  (bind _rotation (.rotation (`self.GetTransform`)))
  (bind _output_get (set `self.timeTravel` (+ (`self.timeTravel`) DeltaSeconds)))
  (if (> _output_get (`self.timeToTravel`))
    (set `self.timeTravel` 0.0)
    (set `self.travelSpeed` (* (`self.travelSpeed`) -1))
    (else
      (`self.K2_SetActorTransform` (`KismetMathLibrary.MakeTransform` (+ (`KismetMathLibrary.MakeVector` (* (.y (`KismetMathLibrary.GetForwardVector` _rotation)) _travelspeed DeltaSeconds -1.0) (* (.x (`KismetMathLibrary.GetForwardVector` _rotation)) _travelspeed DeltaSeconds) (* (.z (`KismetMathLibrary.GetForwardVector` _rotation)) _travelspeed DeltaSeconds -1.0)) (.location (`self.GetTransform`))) (`KismetMathLibrary.MakeRotator` (+ (.roll _rotation) 15.0) (.pitch _rotation) (.yaw _rotation)) (.scale (`self.GetTransform`)))))))

(fn `UserConstructionScript`)