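; CatapultBP is a trap actor that flings the KahnaxChar player when they enter its box trigger.
; Overlap plays a timeline that drives the actor's roll, setting pitch and yaw to zero.
; When it finishes, it passes a scaled arrow forward vector, divided by Tick's DeltaSeconds, to the player's HitByTrap, making the value frame-rate dependent.
; A second timeline then plays with no visible outputs wired.
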(event `self.ReceiveBeginPlay`
  (bind _returnvalue (`GameplayStatics.GetActorOfClass` "/Game/Character/KahnaxChar.KahnaxChar_C"))
  (set `self.player` _returnvalue))

(event `self.Box.OnComponentBeginOverlap`
  (params (OverlappedComponent :type "PrimitiveComponent Object Reference") (OtherActor :type "Actor Object Reference") (OtherComp :type "PrimitiveComponent Object Reference") (OtherBodyIndex :type Integer) (bFromSweep :type Boolean) (SweepResult :type "HitResult Structure (by ref)"))
  (if (== OtherActor (`self.player`))
    (bind (_direction _launch) (`Timeline|Timeline_0`)
      (:`Update`
        (`self.K2_SetActorRotation` (`KismetMathLibrary.MakeRotator` _launch)))
      (:`Finished`
        (`/Game/Character/KahnaxChar.HitByTrap` (`self.player`) (/ (* (`SceneComponent.GetForwardVector` (`self.Arrow`)) (5000.0 5000.0 -5000.0)) (stale `self.ReceiveTick` DeltaSeconds)))
        (`Timeline|Timeline_1`)))))

(event `self.ReceiveTick`
  (params (DeltaSeconds :type "Float (single-precision)")))

(fn `UserConstructionScript`)