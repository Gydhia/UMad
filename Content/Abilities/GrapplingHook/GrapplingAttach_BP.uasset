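; GrapplingAttach_BP is an actor in the grappling hook ability, apparently an attach point, that displays a widget marker.
; The widget hides on BeginPlay, and ShowSelf and HideSelf toggle its visibility along with its children.
; Every Tick it rotates the widget toward the first player's camera manager location, billboarding it.
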(event `self.ReceiveBeginPlay`
  (`self.HideSelf`))

(event `self.ReceiveTick`
  (params (DeltaSeconds :type "Float (single-precision)"))
  (bind _widget (`self.Widget`))
  (`SceneComponent.K2_SetWorldRotation` _widget (`KismetMathLibrary.FindLookAtRotation` (`SceneComponent.K2_GetComponentLocation` _widget) (`SceneComponent.K2_GetComponentLocation` (`PlayerCameraManager.TransformComponent` (`GameplayStatics.GetPlayerCameraManager` 0)))) false false))

(fn `HideSelf`
  (`SceneComponent.SetVisibility` (`self.Widget`) false true))

(fn `ShowSelf`
  (`SceneComponent.SetVisibility` (`self.Widget`) true true))

(fn `UserConstructionScript`)