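; Projectile actor for the primary base attack, moved by a ProjectileMovement component with a 10-second lifespan.
; When its Box hits an actor other than the owner, it prints that actor's name, swaps the projectile particle for the hit particle, stops movement and deactivates the Box.
; It applies no damage and is not explicitly destroyed on impact, leaving cleanup to the lifespan.
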(event `self.ReceiveBeginPlay`
  (`self.SetLifeSpan` 10.0))

(event `self.Box.OnComponentHit`
  (params (HitComponent :type "PrimitiveComponent Object Reference") (OtherActor :type "Actor Object Reference") (OtherComp :type "PrimitiveComponent Object Reference") (NormalImpulse :type "Vector Structure") (Hit :type "HitResult Structure (by ref)"))
  (if (!= OtherActor (`self.GetOwner`))
    (`KismetSystemLibrary.PrintString` (`KismetStringLibrary.Concat_StrStr` "Sent to event : " (`KismetSystemLibrary.GetDisplayName` OtherActor)))
    (`ActorComponent.Activate` (`self.HitParticle`) false)
    (`ActorComponent.Deactivate` (`self.ProjectileParticle`))
    (`MovementComponent.StopMovementImmediately` (`self.ProjectileMovement`))
    (`ActorComponent.Deactivate` (`self.Box`))))

(fn `UserConstructionScript`)