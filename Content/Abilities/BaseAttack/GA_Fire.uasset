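; Gameplay Ability for a three-step primary attack combo that fires a projectile from the hand_r socket on each step.
; Activating mid-attack buffers the input, and a Primary.Hit gameplay event consumes it to spawn the next shot and advance the montage.
; Primary.Reset clears the combo and ends the ability, while another Primary.Hit listener prints the payload target.
; Projectile rotation and scale come from player pawn 0, not the ability's avatar.
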(event `self.K2_ActivateAbility`
  (bind (_returnvalue_owneractor _returnvalue_avataractor _returnvalue_playercontroller _returnvalue_abilitysystemcomponent _returnvalue_skeletalmeshcomponent) (break `GameplayAbilityActorInfo` (`self.GetActorInfo`)))
  (bind (_returnvalue_location _returnvalue_rotation _returnvalue_scale) (`KismetMathLibrary.BreakTransform` (`Actor.GetTransform` (`GameplayStatics.GetPlayerPawn` 0))))
  (bind _returnvalue_location_2 (`KismetMathLibrary.BreakTransform` (`SceneComponent.GetSocketTransform` _returnvalue_skeletalmeshcomponent "hand_r" "RTS_World")))
  (if (`self.IsAttacking`)
    (set `self.SaveAttack` true)
    (else
      (set `self.IsAttacking` true)
      (`|SpawnActorFromClass` "/Game/Abilities/BaseAttack/BP_PrimaryProjectile.BP_PrimaryProjectile_C" (`KismetMathLibrary.MakeTransform` _returnvalue_location_2 _returnvalue_rotation _returnvalue_scale) "Undefined" "OverrideRootScale" null null :!label _label)
      (switch `int` (`self.AttackCount`)
        (:`0`
          (set `self.AttackCount` 1)
          (`|PlayMontage` _returnvalue_skeletalmeshcomponent
            (:`then`
              _)))
        (:`1`
          (set `self.AttackCount` 2)
          (`|PlayMontage` _returnvalue_skeletalmeshcomponent
            (:`then`
              _)))
        (:`2`
          (set `self.AttackCount` 3)
          (`|PlayMontage` _returnvalue_skeletalmeshcomponent
            (:`then`
              _))))
      (`AbilityTask_WaitGameplayEvent.WaitGameplayEvent` (struct :`TagName` "Primary.Hit") null true
        (:`then`
          (`AbilityTask_WaitGameplayEvent.WaitGameplayEvent` (struct :`TagName` "Primary.Reset") null true
            (:`then`
              (bind (_asynctaskproxy _payload) (`AbilityTask_WaitGameplayEvent.WaitGameplayEvent` (struct :`TagName` "Primary.Hit") null true)
                (:`EventReceived`
                  (`KismetSystemLibrary.PrintString` (`KismetStringLibrary.Concat_StrStr` "Hit : " (`KismetStringLibrary.Conv_ObjectToString` (`.Target` (break `GameplayEventData` _payload))))))))
            (:`EventReceived`
              (`self.ResetCombo`))))
        (:`EventReceived`
          (`self.ComboAttackSave`))))))

(event `ComboAttackSave`
  (if (`self.SaveAttack`)
    (set `self.SaveAttack` false)
    (goto _label)))

(event `ResetCombo`
  (set `self.AttackCount` 0)
  (set `self.SaveAttack` false)
  (set `self.IsAttacking` false)
  (`self.K2_EndAbility`))

(event `self.K2_OnEndAbility`
  (params (bWasCancelled :type Boolean)))