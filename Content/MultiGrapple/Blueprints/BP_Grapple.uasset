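; Grapple hook projectile with a cable visual that fires forward, attaches to what it hits and pulls origin, target or both.
; Collision enables once clear of the origin; on hit, it stores a component-relative anchor to follow moving targets.
; Tick applies velocity-damped spring forces beyond the rope length, via interface messages or physics, with optional auto length change.
; It destroys itself on overstretch, forbidden hits or lost line of sight.
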(event `self.ReceiveBeginPlay`
  (`|ExecutionSequence`
    (:`then_0`
      ;[1 1 1] Shoot projectile
      (set `MovementComponent.Velocity` (* (`self.GetActorForwardVector`) (`self.Speed`)) (`self.ProjectileMovement`))
      (set `ProjectileMovementComponent.ProjectileGravityScale` (`self.Gravity`) (`self.ProjectileMovement`)))
    (:`then_1`
      (`|ExecutionSequence`
        (:`then_0`
          ;[1 1 1] Set min snap length
          (set `self.SnapLength` (`KismetMathLibrary.FMax` (`self.MaxRelaxedLength`) (`self.SnapLength`))))
        (:`then_1`
          (`|ExecutionSequence`
            (:`then_0`
              ;[1 1 1] Autopull
              (if (`self.Autopull`)
                (set `self.AutoChange` true)
                (set `self.LengthChangeSpeed` (* (`self.AutopullSpeed`) -1.0))))
            (:`then_1`
              (`|ExecutionSequence`
                (:`then_0`
                  ;[1 1 1] Ignore collision with origin (need to be called from origin as well)
                  (`PrimitiveComponent.IgnoreActorWhenMoving` (`self.Sphere`) (`self.Origin`) true))
                (:`then_1`
                  ;[1 1 1] Line of sight check
                  (if (`self.RequireLineOfSight`)
                    (`KismetSystemLibrary.K2_SetTimerDelegate` (delegate `LineOfSightCheck`) (`self.LineOfSightCheckInterval`) true)))))))))))

(event `LineOfSightCheck`
  (bind _returnvalue (`self.K2_GetActorLocation`))
  ;[1 1 1] Line of sight check
  (bind _origin (message `/Game/MultiGrapple/Blueprints/BI_GrappleOrigin.GetOrigin` (`self.Origin`) self))
  (bind _returnvalue_2 (* (`KismetMathLibrary.Normal` (- _origin _returnvalue)) (`self.LineOfSightCheckOffset`)))
  (bind (_outhit _returnvalue_3) (`KismetSystemLibrary.LineTraceSingleForObjects` (- _origin _returnvalue_2) (+ _returnvalue_2 _returnvalue) (`self.LineOfSightTypes`)))
  (if _returnvalue_3
    (`self.Destroy`)))

(event `self.ReceiveTick`
  (params (DeltaSeconds :type "Float (single-precision)"))
  (`self.GrappleTick` DeltaSeconds))

(event `ChangeLength`
  (params (Change :type "Float (double-precision)"))
  ;[1 1 1] Length change
  (set `self.Length` (`KismetMathLibrary.FClamp` (+ Change (`self.Length`)) 0.0 (`self.MaxRelaxedLength`))))

(event `Destroy`
  (`self.OnDestroy` self)
  (message `/Game/MultiGrapple/Blueprints/BI_GrappleTarget.HookRemoved` (`self.TargetActor`) null)
  (`self.K2_DestroyActor`))

(event `StartLengthChange`
  (params (Speed :type "Float (double-precision)"))
  ;[1 1 1] Length change
  (set `self.AutoChange` true)
  (set `self.LengthChangeSpeed` Speed))

(event `self.Sphere.OnComponentHit`
  (params (HitComponent :type "PrimitiveComponent Object Reference") (OtherActor :type "Actor Object Reference") (OtherComp :type "PrimitiveComponent Object Reference") (NormalImpulse :type "Vector Structure") (Hit :type "HitResult Structure (by ref)"))
  (`self.GrappleHit` OtherActor OtherComp Hit))

(event `StopLengthChange`
  ;[1 1 1] Length change
  (set `self.AutoChange` false)
  (set `self.LengthChangeSpeed` 0.0))

(fn `GrappleHit`
  (params (Actor :type "Actor Object Reference") (Comp :type "PrimitiveComponent Object Reference") (Hit :type "HitResult Structure (by ref)"))
  (bind _comp (`local.Comp`))
  (bind _comp_2 (`local.Comp`))
  (if (!= Actor (`self.Origin`))
    (if (`KismetArrayLibrary.Array_Contains` (`self.DestroyOnHittingTypes`) (`PrimitiveComponent.GetCollisionObjectType` (`local.Comp`)))
      (`self.Destroy`)
      (else
        (`PrimitiveComponent.SetCollisionEnabled` (`self.Sphere`) "NoCollision")
        (`MovementComponent.StopMovementImmediately` (`self.ProjectileMovement`))
        (`|ExecutionSequence`
          (:`then_0`
            ;[1 1 1] Setting target
            (set `self.TargetActor` (`local.Actor`))
            (set `self.TargetComp` _comp)
            (set `self.TargetRelative` (/ (`KismetMathLibrary.LessLess_VectorRotator` (- (`self.K2_GetActorLocation`) (`SceneComponent.K2_GetComponentLocation` _comp)) (`SceneComponent.K2_GetComponentRotation` _comp_2)) (`SceneComponent.K2_GetComponentScale` _comp_2)))
            (set `self.TargetNormal` (`KismetMathLibrary.LessLess_VectorRotator` (* (`.Normal` (`GameplayStatics.BreakHitResult` (`local.Hit`))) -1.0) (`SceneComponent.K2_GetComponentRotation` (`local.Comp`)))))
          (:`then_1`
            (`|ExecutionSequence`
              (:`then_0`
                ;[1 1 1] Register hooked
                (set `self.Hooked` true)
                (`self.OnHooked` self (`self.TargetActor`))
                (message `/Game/MultiGrapple/Blueprints/BI_GrappleTarget.HookAttached` (`self.TargetActor`) self (`self.K2_GetActorLocation`)))
              (:`then_1`
                ;[1 1 1] Set length on hook
                (if (`self.SetLengthOnHook`)
                  (bind _origin (message `/Game/MultiGrapple/Blueprints/BI_GrappleOrigin.GetOrigin` (`self.Origin`) self))
                  (set `self.Length` (`KismetMathLibrary.FMin` (* (`self.HookedLengthRatio`) (`KismetMathLibrary.Vector_Distance` _origin (`self.K2_GetActorLocation`))) (`self.MaxRelaxedLength`)))
                  (else
                    (set `self.Length` (`self.MaxRelaxedLength`))))))))))))

(fn `GrappleTick`
  (params (Delta :type "Float (double-precision)"))
  (locals (OriginPos :type "Vector Structure" :default (0.0 0.0 0.0)) (Distance :type "Float (double-precision)" :default 0.0))
  (bind _targetcomp (`self.TargetComp`))
  (bind _returnvalue (- (`local.OriginPos`) (+ (`self.K2_GetActorLocation`) (* (`SceneComponent.GetComponentVelocity` (`self.TargetComp`)) (- 1.0 (`self.Rubbery`))))))
  (bind _returnvalue_2 (- (`self.K2_GetActorLocation`) (+ (`local.OriginPos`) (* (`self.GetVelocity` (`self.Origin`)) (- 1.0 (`self.Rubbery`))))))
  (bind _origin (message `/Game/MultiGrapple/Blueprints/BI_GrappleOrigin.GetOrigin` (`self.Origin`) self))
  (set `local.OriginPos` _origin)
  (set `local.Distance` (`KismetMathLibrary.Vector_Distance` (`self.K2_GetActorLocation` self) (`local.OriginPos`)))
  (`|ExecutionSequence`
    (:`then_0`
      ;[1 1 1] Refresh Attachment
      (if (`self.Hooked`)
        (`self.K2_SetActorLocationAndRotation` (+ (`SceneComponent.K2_GetComponentLocation` _targetcomp) (`KismetMathLibrary.GreaterGreater_VectorRotator` (* (`self.TargetRelative`) (`SceneComponent.K2_GetComponentScale` _targetcomp)) (`SceneComponent.K2_GetComponentRotation` _targetcomp))) (`KismetMathLibrary.Conv_VectorToRotator` (`KismetMathLibrary.GreaterGreater_VectorRotator` (`self.TargetNormal`) (`SceneComponent.K2_GetComponentRotation` _targetcomp))))))
    (:`then_1`
      (`|ExecutionSequence`
        (:`then_0`
          ;[1 1 1] Visual
          (set `CableComponent.EndLocation` (`KismetMathLibrary.LessLess_VectorRotator` (- (`local.OriginPos`) (`SceneComponent.K2_GetComponentLocation` (`self.Cable`))) (`self.K2_GetActorRotation`)) (`self.Cable`))
          (set `CableComponent.CableLength` (* (`KismetMathLibrary.FMin` (`self.MaxRelaxedLength`) (`local.Distance`)) (`self.VisualStretchModifier`)) (`self.Cable`)))
        (:`then_1`
          (if (`self.Shot`)
            (if (`self.Hooked`)
              ;[1 1 1] Hooked Snap Destroy
              (if (> (`local.Distance`) (`self.SnapLength`))
                (`self.Destroy`)
                (else
                  (`|ExecutionSequence`
                    (:`then_0`
                      ;[1 1 1] Auto change
                      (if (`self.AutoChange`)
                        (`self.ChangeLength` (* (`self.LengthChangeSpeed`) (`local.Delta`)))))
                    (:`then_1`
                      (if (> (`local.Distance`) (`self.Length`))
                        (switch `/Game/MultiGrapple/Blueprints/E_ForceDir` (`self.Direction`)
                          (:`NewEnumerator0`
                            ;[1 1 1] Force on Origin (Player)
                            (message `/Game/MultiGrapple/Blueprints/BI_GrappleOrigin.AddForceOrigin` (`self.Origin`) (* (- _returnvalue_2 (* (`KismetMathLibrary.Normal` _returnvalue_2) (`self.Length`))) (`self.Strength`)) :!label _label))
                          (:`NewEnumerator1`
                            (`|ExecutionSequence` :!label _label_2
                              (:`then_0`
                                ;[1 1 1] Force on component that's simulating physics
                                (if (`self.AffectPhysicsComponents`)
                                  (if (`SceneComponent.IsSimulatingPhysics` (`self.TargetComp`) "None")
                                    (`PrimitiveComponent.AddForceAtLocation` (`self.TargetComp`) (* (- _returnvalue (* (`KismetMathLibrary.Normal` _returnvalue) (`self.Length`))) (`self.Strength`)) (`self.K2_GetActorLocation`) "None"))))
                              (:`then_1`
                                ;[1 1 1] Force on target (interface)
                                (bind _velocity (message `/Game/MultiGrapple/Blueprints/BI_GrappleTarget.GetTargetVelocity` (`self.TargetActor`)))
                                (bind _returnvalue_3 (- (`local.OriginPos`) (+ (* _velocity (- 1.0 (`self.Rubbery`))) (`self.K2_GetActorLocation`))))
                                (message `/Game/MultiGrapple/Blueprints/BI_GrappleTarget.AddForceTarget` (`self.TargetActor`) (* (- _returnvalue_3 (* (`KismetMathLibrary.Normal` _returnvalue_3) (`self.Length`))) (`self.Strength`)) (`self.K2_GetActorLocation`)))))
                          (:`NewEnumerator2`
                            (`|ExecutionSequence`
                              (:`then_0`
                                (goto _label))
                              (:`then_1`
                                (goto _label_2))))))))))
              (else
                ;[1 1 1] Unhooked Destroy
                (if (> (`local.Distance`) (`self.DestroyLength`))
                  (`self.Destroy`))))
            (else
              ;[1 1 1] Enable collision
              (if (> (`local.Distance`) (+ (`self.ActivateCollisionDistance`) (* (`KismetMathLibrary.VSize` (`self.GetVelocity` (`self.Origin`))) (`local.Delta`) (`self.ActivateCollisionVelocityMultiplier`))))
                (set `self.Shot` true)
                (for _array_element (`self.TargetTypes`)
                  (`PrimitiveComponent.SetCollisionResponseToChannel` (`self.Sphere`) _array_element "ECR_Block"))
                (for _array_element_2 (`self.DestroyOnHittingTypes`)
                  (`PrimitiveComponent.SetCollisionResponseToChannel` (`self.Sphere`) _array_element_2 "ECR_Block"))))))))))

(fn `UserConstructionScript`)