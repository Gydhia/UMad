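; UDP networking actor that links the game to a client device on the local network, exchanging player progress, trap info and game-over state.
; Discovery broadcasts the local IP; a received ComputerIP message retargets the send socket and saves the link to the game instance.
; Other messages are colon-delimited strings, with received trap types activating traps through the game instance.
; A looping timer detects player death, notifies the client, shows the game-over menu and pauses.
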(event `self.ReceiveBeginPlay`
  (`KismetSystemLibrary.K2_SetTimerDelegate` (delegate `CheckPlayerState`) 0.5 true)
  (`self.EnableInput` (`GameplayStatics.GetPlayerController` 0))
  (bind _returnvalue (`UDPComponent.GetLocalIPAddress` (`self.UDP_Component`)))
  (`KismetSystemLibrary.PrintString` _returnvalue))

(event `CheckPlayerState`
  (bind _asumad_character (cast `UMadCharacter` (`GameplayStatics.GetPlayerCharacter` 0)))
  (if (and (`UMadCharacter.IsDead` _asumad_character) (not (`self.HasUpdatedPlayerDeath`)))
    (set `self.HasUpdatedPlayerDeath` true)
    (`UDPComponent.EmitBytes` (`self.UDP_Component`) (`CUBlueprintLibrary.Conv_StringToBytes` (`KismetSystemLibrary.MakeLiteralString` (`KismetStringLibrary.Concat_StrStr` "GameOver" ":" "false"))))
    (bind _returnvalue (`|CreateWidget` "/Game/UI/GameOverMenu.GameOverMenu_C"))
    (`UserWidget.AddToViewport` _returnvalue 0)
    (set `PlayerController.bShowMouseCursor` true (`GameplayStatics.GetPlayerController` 0))
    (`GameplayStatics.SetGamePaused` true)
    (`GameplayStatics.PlaySound2D` null 1.0 1.0 0.0 null null)))

(event `self.UDP_Component.OnReceivedBytes`
  (params (Bytes :type "Array of Byte (by ref)") (IPAddress :type String))
  (bind _returnvalue (`CUBlueprintLibrary.Conv_BytesToString` Bytes))
  (bind _udp_component (`self.UDP_Component`))
  (if (`KismetStringLibrary.NotEqual_StrStr` IPAddress (`self.SelfIP`))
    (if (`KismetStringLibrary.Contains` _returnvalue "ComputerIP")
      (bind _output_get (set `self.ClientIP` (`.RightS` (`KismetStringLibrary.Split` _returnvalue ":"))))
      (`UDPComponent.CloseSendSocket` _udp_component)
      (`UDPComponent.OpenSendSocket` _udp_component _output_get (`self.Port`))
      (`KismetSystemLibrary.PrintString` (`KismetStringLibrary.Concat_StrStr` "Client IP set to : " _output_get))
      (set `self.IsLinkedToClient` true)
      (bind _asumad_game_instance (cast `/Game/Network/UMadGameInstance` (`GameplayStatics.GetGameInstance`)))
      (set `/Game/Network/UMadGameInstance.SelfIP` (`self.SelfIP`) _asumad_game_instance)
      (set `/Game/Network/UMadGameInstance.ClientIP` (`self.ClientIP`) _asumad_game_instance)
      (set `/Game/Network/UMadGameInstance.Port` (`self.Port`) _asumad_game_instance)
      (set `/Game/Network/UMadGameInstance.IsLinkedToClient` true _asumad_game_instance)
      (else
        (`self.SortReceivedDatas` _returnvalue)))))

(event `Key|G`
  (params (Key :type "Key Structure"))
  (:`Pressed`
    (`UDPComponent.EmitBytes` (`self.UDP_Component`) (`CUBlueprintLibrary.Conv_StringToBytes` "Datas from next scene"))))

(fn `SendClosestTrap`
  (params (TrapType :type String))
  (`UDPComponent.EmitBytes` (`self.UDP_Component`) (`CUBlueprintLibrary.Conv_StringToBytes` (`KismetStringLibrary.Concat_StrStr` "TrapType:" TrapType))))

(fn `SendCurrentProgress`
  (params (Progress :type "Float (double-precision)"))
  (bind _returnvalue (`KismetStringLibrary.Concat_StrStr` "PlayerProgression:" (`KismetStringLibrary.GetSubstring` (`KismetStringLibrary.Conv_DoubleToString` Progress) 0 4)))
  (`UDPComponent.EmitBytes` (`self.UDP_Component`) (`CUBlueprintLibrary.Conv_StringToBytes` _returnvalue))
  (`KismetSystemLibrary.PrintString` _returnvalue))

(fn `SendHasBuffTrap`
  (`UDPComponent.EmitBytes` (`self.UDP_Component`) (`CUBlueprintLibrary.Conv_StringToBytes` "BuffType:1")))

(fn `SortReceivedDatas`
  (params (Datas :type String))
  (bind (_lefts _rights) (`KismetStringLibrary.Split` Datas ":"))
  (if (`KismetStringLibrary.Contains` _lefts "Traptype")
    (bind _asumad_game_instance (cast `/Game/Network/UMadGameInstance` (`GameplayStatics.GetGameInstance`)))
    (`GameplayStatics.PlaySound2D` "/Game/Sounds/Notification_sound_17.Notification_sound_17" 1.0 1.0 0.0 null null)
    (switch `string` _rights
      (:`0`
        (`/Game/Network/UMadGameInstance.ActivateProjectileTraps` _asumad_game_instance))
      (:`1`
        (`/Game/Network/UMadGameInstance.ActivateKineticTraps` _asumad_game_instance))
      (:`2`
        (`/Game/Network/UMadGameInstance.ActivateElementalTraps` _asumad_game_instance))
      (:`3`
        (`/Game/Network/UMadGameInstance.ActivateBuffTraps` _asumad_game_instance)))))

(fn `TryFindDevice`
  (params (Port :type Integer) (SelfIp :type String))
  (bind _udp_component (`self.UDP_Component`))
  (`UDPComponent.CloseSendSocket` (`self.UDP_Component`))
  (`UDPComponent.OpenSendSocket` _udp_component "255.255.255.255" Port)
  (`UDPComponent.EmitBytes` _udp_component (`CUBlueprintLibrary.Conv_StringToBytes` (`KismetStringLibrary.Concat_StrStr` "ComputerIP:" SelfIp))))

(fn `UserConstructionScript`)