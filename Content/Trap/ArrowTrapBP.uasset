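; Arrow trap actor that automatically and repeatedly fires arrows at a rate set by FireRate.
; Tick accumulates a reload timer, then spawns an ArrowBP at a random point in a scale-sized world X/Z area offset from Base.
; Each arrow takes Base's rotation with an added roll, gets a short lifetime, and is launched along its up vector by an ArrowSpeed impulse divided by frame delta time.
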(event `self.ReceiveBeginPlay`
  (set `self.arrowCooldown` (/ 1.0 (`self.fireRate`))))

(event `self.ReceiveTick`
  (params (DeltaSeconds :type "Float (single-precision)"))
  (if (< (`self.reload`) (`self.arrowCooldown`))
    (set `self.reload` (+ (`self.reload`) DeltaSeconds))
    (else
      (bind _returnvalue (`|SpawnActorFromClass` "/Game/Trap/ArrowBP.ArrowBP_C" (`KismetMathLibrary.MakeTransform` (`KismetMathLibrary.MakeVector` (+ (.x (.location (`SceneComponent.K2_GetComponentToWorld` (`self.Base`)))) (* (+ (* (`KismetMathLibrary.RandomFloat`) 80.0) -40.0) (.y (`self.GetActorScale3D`)))) (+ (.y (.location (`SceneComponent.K2_GetComponentToWorld` (`self.Base`)))) -70.0) (+ (* (+ (* (`KismetMathLibrary.RandomFloat`) 80.0) -40.0) (.x (`self.GetActorScale3D`))) (.z (.location (`SceneComponent.K2_GetComponentToWorld` (`self.Base`)))))) (`KismetMathLibrary.MakeRotator` (+ (.roll (.rotation (`SceneComponent.K2_GetComponentToWorld` (`self.Base`)))) 270.0) (.pitch (.rotation (`SceneComponent.K2_GetComponentToWorld` (`self.Base`)))) (.yaw (.rotation (`SceneComponent.K2_GetComponentToWorld` (`self.Base`))))) (.scale (`SceneComponent.K2_GetComponentToWorld` (`self.Base`)))) "AlwaysSpawn" "OverrideRootScale" self null))
      (set `self.reload` 0.0)
      (set `/Game/Trap/ArrowBP.lifeTime` 2.0 _returnvalue)
      (bind _arrow (`/Game/Trap/ArrowBP.Arrow` _returnvalue))
      (`PrimitiveComponent.AddImpulse` _arrow (/ (* (`KismetMathLibrary.GetUpVector` (`SceneComponent.K2_GetComponentRotation` _arrow)) (`self.arrowSpeed`)) DeltaSeconds) "None" false))))

(fn `UserConstructionScript`)