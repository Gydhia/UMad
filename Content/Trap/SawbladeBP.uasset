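; Sawblade trap that shuttles back and forth along a straight path while spinning.
; BeginPlay derives the leg duration from travel distance and speed, and Tick flips the speed sign whenever that time elapses.
; Otherwise Tick moves it sideways, using swizzled forward-vector components, and adds a fixed roll per frame, so spin depends on frame rate.
; The overlap event is empty, so no damage is handled here.
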(event `self.ReceiveBeginPlay`
  (set `self.timeTravel` 0.0)
  (set `self.timeToTravel` (/ (`self.distanceToTravel`) (`self.travelSpeed`))))

(event `self.ReceiveTick`
  (params (DeltaSeconds :type "Float (single-precision)"))
  (bind _travelspeed (`self.travelSpeed`))
  (bind _rotation (.rotation (`self.GetTransform`)))
  (bind _output_get (set `self.timeTravel` (+ (`self.timeTravel`) DeltaSeconds)))
  (if (> _output_get (`self.timeToTravel`))
    (set `self.timeTravel` 0.0)
    (set `self.travelSpeed` (* (`self.travelSpeed`) -1))
    (else
      (`self.K2_SetActorTransform` (`KismetMathLibrary.MakeTransform` (+ (`KismetMathLibrary.MakeVector` (* (.y (`KismetMathLibrary.GetForwardVector` _rotation)) _travelspeed DeltaSeconds -1.0) (* (.x (`KismetMathLibrary.GetForwardVector` _rotation)) _travelspeed DeltaSeconds) (* (.z (`KismetMathLibrary.GetForwardVector` _rotation)) _travelspeed DeltaSeconds -1.0)) (.location (`self.GetTransform`))) (`KismetMathLibrary.MakeRotator` (+ (.roll _rotation) 15.0) (.pitch _rotation) (.yaw _rotation)) (.scale (`self.GetTransform`)))))))

(fn `UserConstructionScript`)